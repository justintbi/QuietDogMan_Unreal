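; Coworker actor that turns to watch the player and reacts to having its butt sniffed.
; Each tick, while the player overlaps its detection sphere and is neither sneaking nor sniffing, it rotates to face them without pitching.
; ButtSniffed destroys the sphere, ending that tracking, and sets CheckVis.
; CheckVis shows a Paper sprite that Tick billboards toward the camera with a yaw offset.
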(event `self.ReceiveTick`
  (params (DeltaSeconds :type "Float (single-precision)"))
  (bind _papersprite (`self.PaperSprite`))
  (bind _sphere (`self.Sphere`))
  (bind (_returnvalue_roll _returnvalue_pitch _returnvalue_yaw) (`KismetMathLibrary.BreakRotator` (`KismetMathLibrary.FindLookAtRotation` (`self.K2_GetActorLocation`) (`self.K2_GetActorLocation` (`GameplayStatics.GetPlayerCameraManager` 0)))))
  ;[1 1 1] Sphere Detection
  (`/Engine/EditorBlueprintResources/StandardMacros.IsValid` _sphere
    (:`Is Valid`
      (if (`PrimitiveComponent.IsOverlappingActor` _sphere (`GameplayStatics.GetPlayerCharacter` 0))
        (bind _asthird_person_character (cast `/Game/ThirdPersonBP/Blueprints/ThirdPersonCharacter` (`GameplayStatics.GetPlayerCharacter` 0)))
        (if (not (or (`/Game/ThirdPersonBP/Blueprints/ThirdPersonCharacter.IsSneaking` _asthird_person_character) (`/Game/ThirdPersonBP/Blueprints/ThirdPersonCharacter.IsSniffing` _asthird_person_character)))
          (`self.K2_SetActorRotation` (`KismetMathLibrary.MakeRotator` (.roll (`KismetMathLibrary.FindLookAtRotation` (`self.K2_GetActorLocation`) (`self.K2_GetActorLocation` (`GameplayStatics.GetPlayerCharacter` 0)))) 0.0 (.yaw (`KismetMathLibrary.FindLookAtRotation` (`self.K2_GetActorLocation`) (`self.K2_GetActorLocation` (`GameplayStatics.GetPlayerCharacter` 0)))))))))
    (:`Is Not Valid`
      _))
  (if (`self.CheckVis`)
    (`SceneComponent.SetVisibility` _papersprite true false)
    (`SceneComponent.K2_SetWorldRotation` (`self.PaperSprite`) (`KismetMathLibrary.MakeRotator` _returnvalue_roll _returnvalue_pitch (- _returnvalue_yaw 90.0)) false false)
    (else
      (`SceneComponent.SetVisibility` _papersprite false false))))

(event `/Game/Blueprints/BPI.ButtSniffed`
  (`ActorComponent.K2_DestroyComponent` (`self.Sphere`))
  (set `self.CheckVis` true))

(fn `UserConstructionScript`)