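; CoworkerAI is an AI controller for a coworker NPC that can catch the player sniffing.
; It runs the CoworkerBT behavior tree and uses AI perception to write CanSeePlayer to the blackboard for ThirdPersonCharacter, with debug prints.
; The local sight flag updates before the cast, so any perceived actor changes it.
; AlertCoworkerToSniff sets CoworkerHasCaughtSniffing only while that flag is true, and nothing here clears it.
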(event `self.ReceiveBeginPlay`
  (`self.RunBehaviorTree` "/Game/Blueprints/CoworkerBT.CoworkerBT"))

(event `self.AIPerception.OnTargetPerceptionUpdated`
  (params (Actor :type "Actor Object Reference") (Stimulus :type "AIStimulus Structure"))
  (bind _output_get (set `self.CanSeePlayer` Stimulus_bSuccessfullySensed))
  (cast `/Game/ThirdPersonBP/Blueprints/ThirdPersonCharacter` Actor)
  (if _output_get
    (`KismetSystemLibrary.PrintString` "Spotted")
    (else
      (`KismetSystemLibrary.PrintString` "Hidden")))
  (`BlackboardComponent.SetValueAsBool` (`AIBlueprintHelperLibrary.GetBlackboard` null) "CanSeePlayer" _output_get))

(event `AlertCoworkerToSniff`
  (bind _canseeplayer (`self.CanSeePlayer`))
  (if _canseeplayer
    (`BlackboardComponent.SetValueAsBool` (`AIBlueprintHelperLibrary.GetBlackboard` null) "CoworkerHasCaughtSniffing" _canseeplayer)))

(fn `UserConstructionScript`)